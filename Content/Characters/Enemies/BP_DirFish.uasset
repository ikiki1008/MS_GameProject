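; BP_DirFish is a fish enemy Blueprint that plays animation montages on its mesh for idle, run, attack, hit and death.
; Custom events each play one montage, and the Attacking, Idle and Dead functions call their matching events.
; The Hit function calls StartRun instead of HitByPlayer, the Run function is empty, and nothing in this file calls HitByPlayer.
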(event `StartRun`
  (`|PlayMontage` (`self.Mesh`) "/Game/Characters/Enemies/Assets/Luminous_Monster/Mesh/FIsh_Run_Montage.FIsh_Run_Montage"))

(event `StartAttack`
  (`|PlayMontage` (`self.Mesh`) "/Game/Characters/Enemies/Assets/Luminous_Monster/Mesh/Fish_Attack_Montage.Fish_Attack_Montage"))

(event `StartIdle`
  (`|PlayMontage` (`self.Mesh`) "/Game/Characters/Enemies/Assets/Luminous_Monster/Mesh/FIsh_Idle_Montage.FIsh_Idle_Montage"))

(event `Die`
  (`|PlayMontage` (`self.Mesh`) "/Game/Characters/Enemies/Assets/Luminous_Monster/Mesh/Fish_Dead_Montage.Fish_Dead_Montage"))

(event `HitByPlayer`
  (`|PlayMontage` (`self.Mesh`) "/Game/Characters/Enemies/Assets/Luminous_Monster/Mesh/Fish_Hit_Montage.Fish_Hit_Montage"))

(fn `Attacking`
  (`self.StartAttack`))

(fn `Dead`
  (`self.Die`))

(fn `Hit`
  (`self.StartRun`))

(fn `Idle`
  (`self.StartIdle`))

(fn `Run`)

(fn `UserConstructionScript`)