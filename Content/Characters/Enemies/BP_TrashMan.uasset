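; BP_TrashMan is an enemy character that responds to behavior states with rat montages and a leap attack.
; Attacking, Idle and Dead functions forward to matching events, while Run and Hit are empty, leaving StartRun uncalled within this graph.
; The attack jumps, launches the character using the player's world location as the velocity, then stops jumping.
; Hit and death events are stubs.
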(event `StartRun`
  (`|PlayMontage` (`self.Mesh`) "/Game/Characters/Enemies/Assets/Rat/Meshes/RatRunMontage.RatRunMontage"))

(event `HitbyPlayer`)

(event `StartAttack`
  (`self.Jump`)
  (`self.LaunchCharacter` (`self.K2_GetActorLocation` (`GameplayStatics.GetPlayerCharacter` 0)))
  (`self.StopJumping`))

(event `StartIdle`
  (`|PlayMontage` (`self.Mesh`) "/Game/Characters/Enemies/Assets/Rat/Meshes/RatIdleMontage.RatIdleMontage"))

(event `Died`)

(fn `Attacking`
  (`self.StartAttack`))

(fn `Dead`
  (`self.Died`))

(fn `Hit`)

(fn `Idle`
  (`self.StartIdle`))

(fn `Run`)

(fn `UserConstructionScript`)